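; BP_Target is a moving shootable target that patrols back and forth and is destroyed after enough hits.
; Tick offsets it along the normalized Direction by Speed each frame, without delta-time scaling or sweeping.
; A looping timer set on BeginPlay reverses Direction every MovementDuration seconds.
; The Hit event decrements HP and destroys the actor once it reaches zero.
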(event `self.ReceiveBeginPlay`
  ;[0.04374 0.4397 0.3515 0.502] FlipDirection1
  (`KismetSystemLibrary.K2_SetTimerDelegate` (delegate `FlipDirection`) (`self.MovementDuration`) true))

(event `self.ReceiveTick`
  (params (DeltaSeconds :type "Float (single-precision)"))
  ;[0.04374 0.4397 0.3515 0.502] TargetMovementBlock1
  (`self.K2_AddActorWorldOffset` (* (`KismetMathLibrary.Normal` (`self.Direction`)) (`self.Speed`))))

(event `FlipDirection`
  ;[0.04374 0.4397 0.3515 0.502] FlipDirection2
  (set `self.Direction` (* (`self.Direction`) -1.0)))

(event `self.ReceiveHit`
  (params (MyComp :type "PrimitiveComponent Object Reference") (Other :type "Actor Object Reference") (OtherComp :type "PrimitiveComponent Object Reference") (bSelfMoved :type Boolean) (HitLocation :type "Vector Structure") (HitNormal :type "Vector Structure") (NormalImpulse :type "Vector Structure") (Hit :type "HitResult Structure (by ref)"))
  (set `self.HP` (- (`self.HP`) 1))
  (if (<= (`self.HP`) 0)
    (`self.K2_DestroyActor`)))

(fn `UserConstructionScript`)