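; BP_Door is a key-locked door that swings open for the player and shows its lock state on a light.
; On BeginPlay it caches the first-person character and gives the door light a dynamic material instance.
; When the player enters the trigger, the light brightens, turning green and playing a rotation timeline if they hold the key, or red otherwise.
; Leaving the trigger restores the default light and reverses the timeline to close the door.
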(event `self.ReceiveBeginPlay`
  ; Retrieval
  (bind _asbp_first_person_character (cast `/Game/TheVibes/Blueprints/BP_FirstPersonCharacter` (`GameplayStatics.GetPlayerCharacter` 0)))
  (set `self.Player` _asbp_first_person_character)
  (bind _returnvalue (`KismetMaterialLibrary.CreateDynamicMaterialInstance` "/Game/TheVibes/Materials/MI_LIGHTEMUP_DoorLight.MI_LIGHTEMUP_DoorLight"))
  (bind _output_get (set `self.DynamicMaterial` _returnvalue))
  (`PrimitiveComponent.SetMaterial` (`self.SM_Doorlight`) 0 _output_get))

(event `self.DoorTrigger.OnComponentBeginOverlap`
  (params (OverlappedComponent :type "PrimitiveComponent Object Reference") (OtherActor :type "Actor Object Reference") (OtherComp :type "PrimitiveComponent Object Reference") (OtherBodyIndex :type Integer) (bFromSweep :type Boolean) (SweepResult :type "HitResult Structure (by ref)"))
  ; Door-LightFunction
  (if (== OtherActor (`self.Player`))
    (`MaterialInstanceDynamic.SetScalarParameterValue` (`self.DynamicMaterial`) "Intensity" 100.0)
    (if (`/Game/TheVibes/Blueprints/BP_FirstPersonCharacter.HasKey` (`self.Player`))
      (`MaterialInstanceDynamic.SetVectorParameterValue` (`self.DynamicMaterial`) "Colour" (struct :`R` 0.317558 :`G` 1.0 :`B` 0.054441 :`A` 1.0))
      ; DoorAnimation
      (bind (_direction _alpha) (`Timeline|Timeline` :!label _label)
        (:`Update`
          (`SceneComponent.K2_SetRelativeRotation` (`self.SM_Door`) (`KismetMathLibrary.RLerp` (struct) (struct :`Yaw` 90.0) _alpha) false false)))
      (else
        (`MaterialInstanceDynamic.SetVectorParameterValue` (`self.DynamicMaterial`) "Colour" (struct :`R` 1.0 :`G` 0.054441 :`B` 0.127094 :`A` 1.0))))))

(event `self.DoorTrigger.OnComponentEndOverlap`
  (params (OverlappedComponent :type "PrimitiveComponent Object Reference") (OtherActor :type "Actor Object Reference") (OtherComp :type "PrimitiveComponent Object Reference") (OtherBodyIndex :type Integer))
  ; ReturnLightToDefault
  (if (== OtherActor (`self.Player`))
    (`MaterialInstanceDynamic.SetScalarParameterValue` (`self.DynamicMaterial`) "Intensity" 1.0)
    (`MaterialInstanceDynamic.SetVectorParameterValue` (`self.DynamicMaterial`) "Colour" (struct :`R` 0.364818 :`G` 1.0 :`B` 0.888603 :`A` 1.0))
    (goto _label :!via `Reverse`)))

(fn `UserConstructionScript`)