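; BP_Cmaera is a security camera for a stealth level that sweeps back and forth and catches the first-person player.
; A looping MoveCamera event uses a FlipFlop to rotate the camera mesh between start and end rotations, pausing between moves.
; Every Tick, Detect traces forward from SMLineTrace for pawns, drawing a debug line.
; A hit on the player prints a message, disables input and opens SneakyMap after a delay.
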(event `self.ReceiveBeginPlay`
  ; Player ref
  (`self.moveCamera`)
  (bind _asbp_first_person_character (cast `/Game/TheVibes/Blueprints/BP_FirstPersonCharacter` (`GameplayStatics.GetPlayerCharacter` 0)))
  (set `self.PLayer ref` _asbp_first_person_character))

(event `moveCamera`
  (bind (_current_rotation_roll _current_rotation_pitch _current_rotation_yaw) (`KismetMathLibrary.BreakRotator` (`self.current rotation`)))
  ; MoveCamera
  (`/Engine/EditorBlueprintResources/StandardMacros.FlipFlop`
    (:`A`
      (set `self.current rotation` (`self.EndRotation`)))
    (:`B`
      (set `self.current rotation` (`self.StartRotation`))))
  (`KismetSystemLibrary.MoveComponentTo` (`self.SM_SecurityCam`) (0.0 0.0 0.0) (`KismetMathLibrary.MakeRotator` _current_rotation_roll _current_rotation_pitch _current_rotation_yaw) false false (`self.speed`))
  (`KismetSystemLibrary.Delay` (`self.delay`))
  (`self.moveCamera`))

(event `Detect`
  (bind _sm_linetrace (`self.SM_LineTrace`))
  (bind _returnvalue (`SceneComponent.K2_GetComponentLocation` _sm_linetrace))
  ; Detection
  (bind _outhit (`KismetSystemLibrary.LineTraceSingleForObjects` :`Start` _returnvalue :`End` (+ _returnvalue (* (`KismetMathLibrary.GetForwardVector` (`SceneComponent.K2_GetComponentRotation` _sm_linetrace)) (`self.DetectDistance`))) :`ObjectTypes` (`|MakeArray` "ObjectTypeQuery3" :!type "EObjectTypeQuery Enum") :`DrawDebugType` "ForOneFrame" :`TraceColor` (struct :`R` 0.848958 :`G` 0.13288 :`A` 1.0) :`TraceHitColor` (struct :`G` 0.848958 :`B` 0.598509 :`A` 1.0)))
  (if (== (`.HitActor` (`GameplayStatics.BreakHitResult` _outhit)) (`self.PLayer ref`))
    (`KismetSystemLibrary.PrintString` ":) FOUND YOU :)" true true (struct :`R` 1.0 :`A` 1.0))
    (`self.DisableInput` (`self.PLayer ref`) (`GameplayStatics.GetPlayerController` 0))
    (`KismetSystemLibrary.Delay` (`self.delay`))
    (`GameplayStatics.OpenLevel` "SneakyMap")))

(event `self.ReceiveTick`
  (params (DeltaSeconds :type "Float (single-precision)"))
  ; Detection
  (`self.Detect`))

(fn `UserConstructionScript`)