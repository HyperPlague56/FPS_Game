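; BP_Cake is a spinning pickup that gives the player the cake.
; Tick applies a local rotation each frame, and BeginPlay caches the player's BP_FirstPersonCharacter.
; When that character overlaps the Collision component, it sets HasCake on the character, plays an explosion sound at the player's location and destroys itself.
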(event `self.ReceiveTick`
  (params (DeltaSeconds :type "Float (single-precision)"))
  (`self.K2_AddActorLocalRotation` (`self.Spin`)))

(event `self.ReceiveBeginPlay`
  ; PlayerReference
  (bind _asbp_first_person_character (cast `/Game/TheVibes/Blueprints/BP_FirstPersonCharacter` (`GameplayStatics.GetPlayerCharacter` 0)))
  (set `self.As BP First Person Character` _asbp_first_person_character))

(event `self.collision.OnComponentBeginOverlap`
  (params (OverlappedComponent :type "PrimitiveComponent Object Reference") (OtherActor :type "Actor Object Reference") (OtherComp :type "PrimitiveComponent Object Reference") (OtherBodyIndex :type Integer) (bFromSweep :type Boolean) (SweepResult :type "HitResult Structure (by ref)"))
  ; CakeCollection
  (if (== OtherActor (`self.As BP First Person Character`))
    (set `/Game/TheVibes/Blueprints/BP_FirstPersonCharacter.HasCake` true (`self.As BP First Person Character`))
    (`GameplayStatics.SpawnSoundAtLocation` "/Game/TheVibes/SoundEffects/MP3_Explosion_Big.MP3_Explosion_Big" (`self.K2_GetActorLocation` (`self.As BP First Person Character`)) (struct) 1.0 1.0 0.0 null null)
    (`self.K2_DestroyActor`)))

(fn `UserConstructionScript`)